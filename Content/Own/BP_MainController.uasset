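; BP_MainController is the player-controlled character, handling movement, jumping, coin pickup and triggering enemy spawns.
; It adds the main Enhanced Input mapping context on BeginPlay and moves relative to control rotation while AbleMovement is true.
; Overlapping a coin calls that coin's CoinCollected.
; Tick polls CoinsToSpawn and, once it reaches the threshold, resets it and calls SpawnEnemys on BP_MainGamemode.
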(event Input|EnhancedActionEvents|EnhancedInputActionIA_MainMovement
  (params (ActionValue :type Vector%202D%20Structure) (ElapsedSeconds :type Float%20%28double-precision%29) (TriggeredSeconds :type Float%20%28double-precision%29) (InputAction :type Input%20Action%20Object%20Reference :default "/Game/Own/Movement/IA_MainMovement.IA_MainMovement"))
  (bind _returnvalue (Pawn|GetControlRotation :!class /Script/Engine.Pawn))
  ;[1 1 1] Movement Controller
  (if (Variables|Default|GetableMovement)
    (Utilities|FlowControl|Sequence
      (:then_0
        (Pawn|Input|AddMovementInput (Math|Vector|GetForwardVector (Math|Rotator|MakeRotator 0.0 0.0 (.yaw (Pawn|GetControlRotation :!class /Script/Engine.Pawn)))) (.y ActionValue) false))
      (:then_1
        (Pawn|Input|AddMovementInput (Math|Vector|GetRightVector (Math|Rotator|MakeRotator (.roll _returnvalue) 0.0 (.yaw _returnvalue))) (.x ActionValue) false)))))

(event Input|EnhancedActionEvents|EnhancedInputActionIA_JumpMovement
  (params (ActionValue :type Boolean) (ElapsedSeconds :type Float%20%28double-precision%29) (TriggeredSeconds :type Float%20%28double-precision%29) (InputAction :type Input%20Action%20Object%20Reference :default "/Game/Own/Movement/IA_JumpMovement.IA_JumpMovement"))
  ;[1 1 1] Movement Controller
  ;;[1 1 1] Jump Controller
  (Character|Jump))

(event EventTick
  (params (DeltaSeconds :type Float%20%28single-precision%29))
  ;[1 1 1] EnemySpawner
  (bind _output_get (Variables|Default|SetableSpawn (>= (Variables|Default|GetcoinsToSpawn) 10)))
  (if _output_get
    (Variables|Default|SetcoinsToSpawn 0)
    (bind _asbp_main_gamemode (Utilities|Casting|CastToBP_MainGamemode (Game|GetGameMode)))
    (Default|SpawnEnemys _asbp_main_gamemode)))

(event EventBeginPlay
  ;[1 1 1] GetPlayerController
  (Input|AddMappingContext (PlayerController|LocalPlayerSubsystems|GetEnhancedInputLocalPlayerSubsystem (Game|GetPlayerController 0)) "/Game/Own/Movement/IMC_MainMappingContext.IMC_MainMappingContext" 0 "(bIgnoreAllPressedKeysUntilRelease=True,bForceImmediately=False,bNotifyUserSettings=False)"))

(event Collision|EventActorBeginOverlap
  (params (OtherActor :type Actor%20Object%20Reference))
  ;[1 1 1] CoinCollector
  (bind _asbp_a_coin (Utilities|Casting|CastToBP_A_Coin OtherActor))
  (Default|CoinCollected _asbp_a_coin))

(fn ConstructionScript)