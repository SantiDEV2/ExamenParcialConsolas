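; Collectible coin actor that spins by a fixed local rotation each tick, independent of delta time.
; CoinCollected, not called within this Blueprint, casts the player character to BP_MainController and increments its CoinsToSpawn count.
; It then destroys the coin and tells BP_CoinSpawner to spawn coins.
; Afterwards it increments CoinsCollected on the player and prints the new total.
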(event EventBeginPlay)

(event Collision|EventActorBeginOverlap
  (params (OtherActor :type Actor%20Object%20Reference)))

(event EventTick
  (params (DeltaSeconds :type Float%20%28single-precision%29))
  (Transformation|AddActorLocalRotation self "0.000000,2.000000,0.000000" false false))

(fn ConstructionScript)

(fn CoinCollected
  (bind _asbp_main_controller (Utilities|Casting|CastToBP_MainController (Game|GetPlayerCharacter 0)))
  (Utilities|FlowControl|Sequence
    (:then_0
      (Variables|/Game/Own/BP_MainController.BP_MainController_C|SetcoinsToSpawn _asbp_main_controller (+ (Variables|/Game/Own/BP_MainController.BP_MainController_C|GetcoinsToSpawn _asbp_main_controller) 1))
      (Actor|DestroyActor)
      (bind _returnvalue (Actor|GetActorOfClass "/Game/Own/Coins/BP_CoinSpawner.BP_CoinSpawner_C"))
      (Default|SpawnCoins _returnvalue))
    (:then_1
      (bind _output_get (Variables|/Game/Own/BP_MainController.BP_MainController_C|SetcoinsCollected _asbp_main_controller (+ (Variables|/Game/Own/BP_MainController.BP_MainController_C|GetcoinsCollected _asbp_main_controller) 1)))
      (Development|PrintString (Utilities|String|ToString(Integer) _output_get)))))