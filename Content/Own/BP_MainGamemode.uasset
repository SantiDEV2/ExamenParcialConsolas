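; Main game mode Blueprint that provides enemy spawning through its SpawnEnemys function.
; Each call gathers all BP_EnemySpawnPoint actors in the level, picks one at random and spawns a single BP_C_Enemy at its location.
; The spawn ignores the point's rotation and scale, adjusting for collisions where possible but always spawning.
; Nothing in this graph calls the function, and a leftover debug print is unconnected.
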(fn ConstructionScript)

(fn SpawnEnemys
  (bind _outactors (Actor|GetAllActorsOfClass "/Game/Own/Enemys/BP_EnemySpawnPoint.BP_EnemySpawnPoint_C"))
  (LocalVariables|SetlocalSpawnPoints _outactors)
  (LocalVariables|Setlocalitem (.OutItem (Utilities|Array|Random (LocalVariables|GetlocalSpawnPoints))))
  (Game|SpawnActorfromClass "/Game/Own/Enemys/BP_C_Enemy.BP_C_Enemy_C" (Math|Transform|MakeTransform (Transformation|GetActorLocation (LocalVariables|Getlocalitem))) "AdjustIfPossibleButAlwaysSpawn" "MultiplyWithRoot" 0 0))